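; Purchasable pickup point that sells the player extra respawn lives for Skulls from a limited stock.
; Overlap shows or clears a buy prompt through BPI_Score.
; Buy plays a sound, messages the player to add a life and deduct Skulls, then decrements stock and adjusts the price or reports none left.
; Buy itself checks nothing; CanBuyLife? tests stock and Skulls, while CanBuy? always returns false.
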(event EventBeginPlay
  (Variables|Default|SetDisplay%20String "Press F To Buy 1 Life (respawn when killed)"))

(event EventTick
  (params (DeltaSeconds :type Float%20%28single-precision%29)))

(event Collision|EventActorEndOverlap
  (params (OtherActor :type Actor%20Object%20Reference))
  (if (Utilities|DoesObjectImplementInterface OtherActor "/Game/Blueprints/Interfaces/BPI_Score.BPI_Score_C")
    (Class|BPIScore|DisplayPrompt(Message) OtherActor)))

(event Collision|EventActorBeginOverlap
  (params (OtherActor :type Actor%20Object%20Reference))
  (if (and (!= (Variables|Default|GetLives) 0) (Utilities|DoesObjectImplementInterface OtherActor "/Game/Blueprints/Interfaces/BPI_Score.BPI_Score_C"))
    (Class|BPIScore|DisplayPrompt(Message) OtherActor (Utilities|String|Append (Variables|Default|GetDisplay%20String) " 
" "Cost [" (Utilities|String|ToString(Integer) (Variables|Default|GetCost)) " Skulls]"))
    (else
      (Class|BPIScore|DisplayPrompt(Message) OtherActor "No Lives Remaing"))))

(event EventBuy
  (params (Player :type Actor%20Object%20Reference))
  (Audio|PlaySoundatLocation "/Game/Free_Sounds_Pack/cue/Magical_Interface_8-1_Cue.Magical_Interface_8-1_Cue" (Transformation|GetActorLocation) "0, 0, 0" 1.0 1.0 0.0 0 0 0 0)
  (Class|BPIScore|AddLives(Message) Player)
  (Class|BPIScore|AddSkulls(Message) Player (* (Variables|Default|GetCost) -1))
  (bind _result (Math|Integer|DecrementInt (Variables|Default|GetLives))
    (:%20%20
      (bind _output_get (Variables|Default|SetLives _result))
      (switch int _output_get
        (:0
          (Class|BPIScore|DisplayPrompt(Message) Player "No Lives Remaining"))
        (:1
          (Variables|Default|SetCost 200)
          (Class|BPIScore|DisplayPrompt(Message) Player (Utilities|String|Append (Variables|Default|GetDisplay%20String) " 
" "Cost [" (Utilities|String|ToString(Integer) (Variables|Default|GetCost)) " Skulls]")))
        (:2
          (Variables|Default|SetCost 100)
          (Class|BPIScore|DisplayPrompt(Message) Player (Utilities|String|Append (Variables|Default|GetDisplay%20String) " 
" "Cost [" (Utilities|String|ToString(Integer) (Variables|Default|GetCost)) " Skulls]")))))))

(fn ConstructionScript)

(fn CanBuy?
  (params (CurrentPoints :type Integer))
  (return false))

(fn CanBuyLife?
  (params (Skulls :type Integer))
  (return (and (!= (Variables|Default|GetLives) 0) (>= Skulls (Variables|Default|GetCost)))))