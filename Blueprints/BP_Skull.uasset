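; BP_Skull is a collectible skull pickup that adds to the score of the actor that touches it.
; A fast looping timer, rather than Tick, spins the root component around yaw, and a limited lifespan removes uncollected skulls.
; When an actor implementing BPI_Score overlaps the Sphere, it receives one skull through the interface, a coin sound plays and the pickup destroys itself.
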(event OnComponentBeginOverlap(Sphere)
  (params (OverlappedComponent :type Primitive%20Component%20Object%20Reference) (OtherActor :type Actor%20Object%20Reference) (OtherComp :type Primitive%20Component%20Object%20Reference) (OtherBodyIndex :type Integer) (bFromSweep :type Boolean) (SweepResult :type Hit%20Result%20Structure%20%28by%20ref%29))
  (if (Utilities|DoesObjectImplementInterface OtherActor "/Game/Blueprints/Interfaces/BPI_Score.BPI_Score_C")
    (Class|BPIScore|AddSkulls(Message) OtherActor 1)
    (Audio|PlaySoundatLocation "/Game/Free_Sounds_Pack/cue/Coins_2-1_Cue.Coins_2-1_Cue" (Transformation|GetActorLocation) "0, 0, 0" 1.0 1.0 0.0 0 0 0 0)
    (Actor|DestroyActor)))

(event EventBeginPlay
  (Utilities|Time|SetTimerbyFunctionName 0 "Rotate" 0.005 true)
  (Actor|SetLifeSpan 25.0))

(event Collision|EventActorBeginOverlap
  (params (OtherActor :type Actor%20Object%20Reference)))

(event EventTick
  (params (DeltaSeconds :type Float%20%28single-precision%29)))

(fn ConstructionScript)

(fn Rotate
  (Transformation|AddLocalRotation (Variables|Default|GetDefaultSceneRoot) (Math|Rotator|MakeRotator 0.0 0.0 0.5) false false))