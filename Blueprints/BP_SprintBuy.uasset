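; BP_SprintBuy is a purchasable pickup that sells the player a permanent sprint upgrade for points.
; Overlap shows a buy prompt with the cost, or an already-owned message, through BPI_Score, and leaving clears it.
; CanBuy checks points against Cost and a one-time HasBought flag, while Buy grants the upgrade, deducts points and plays a sound.
; CanBuyLife always returns false, so skulls cannot purchase it.
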(event EventBeginPlay
  (Variables|Default|SetDisplay%20String "Hold  F  To Buy Perma-Sprint"))

(event EventTick
  (params (DeltaSeconds :type Float%20%28single-precision%29)))

(event Collision|EventActorEndOverlap
  (params (OtherActor :type Actor%20Object%20Reference))
  (if (Utilities|DoesObjectImplementInterface OtherActor "/Game/Blueprints/Interfaces/BPI_Score.BPI_Score_C")
    (Class|BPIScore|DisplayPrompt(Message) OtherActor)))

(event Collision|EventActorBeginOverlap
  (params (OtherActor :type Actor%20Object%20Reference))
  (if (and (not (Variables|Default|GetHasBought)) (Utilities|DoesObjectImplementInterface OtherActor "/Game/Blueprints/Interfaces/BPI_Score.BPI_Score_C"))
    (Class|BPIScore|DisplayPrompt(Message) OtherActor (Utilities|String|Append (Variables|Default|GetDisplay%20String) " 
Cost  [" (Utilities|String|ToString(Integer) (Variables|Default|GetCost)) "]"))
    (else
      (Class|BPIScore|DisplayPrompt(Message) OtherActor "Already Have Perma-Sprint"))))

(event EventBuy
  (params (Player :type Actor%20Object%20Reference))
  (Class|BPIScore|UpgradeSprint(Message) Player)
  (Class|BPIScore|TakePoints(Message) Player (Variables|Default|GetCost))
  (Audio|PlaySoundatLocation "/Game/Interface_And_Item_Sounds/Cues/Abstract_Pop_02_Cue.Abstract_Pop_02_Cue" (Transformation|GetActorLocation) "0, 0, 0" 1.0 1.0 0.0 0 0 0 0)
  (Variables|Default|SetHasBought true))

(fn ConstructionScript)

(fn CanBuy?
  (params (CurrentPoints :type Integer))
  (return (and (>= CurrentPoints (Variables|Default|GetCost)) (not (Variables|Default|GetHasBought)))))

(fn CanBuyLife?
  (params (Skulls :type Integer))
  (return false))