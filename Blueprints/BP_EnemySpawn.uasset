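; BP_EnemySpawn is an enemy spawn point actor that shows whether it is active and supplies a spawn transform.
; BeginPlay caches the cube's original material as the inactive look and clears the SpawnOpening audio component's sound.
; SetActive swaps to the active material and plays the opening sound, while SetInactive restores only the material.
; GetLocation returns the SpawnLocation component's world location as a transform; spawning itself happens outside this Blueprint.
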(event EventBeginPlay
  (bind _cube (Variables|Default|GetCube))
  (bind _output_get (Variables|Default|SetInactiveMaterial (Rendering|Material|GetMaterial _cube 0)))
  (Rendering|Material|SetMaterial _cube 0 _output_get)
  (Audio|Components|Audio|SetSound (Variables|Default|GetspawnOpening) 0))

(event Collision|EventActorBeginOverlap
  (params (OtherActor :type Actor%20Object%20Reference)))

(event EventTick
  (params (DeltaSeconds :type Float%20%28single-precision%29)))

(event EventSetActive
  (bind _spawnopening (Variables|Default|GetspawnOpening))
  (Rendering|Material|SetMaterial (Variables|Default|GetCube) 0 (Variables|Default|GetActiveMaterial))
  (Audio|Components|Audio|SetSound _spawnopening "/Game/Soundfx/Spawner/spawnOpening.spawnOpening")
  (Audio|Components|Audio|Play _spawnopening 0.0))

(event EventSetInactive
  (Rendering|Material|SetMaterial (Variables|Default|GetCube) 0 (Variables|Default|GetInactiveMaterial)))

(fn ConstructionScript)

(fn GetLocation
  (return (Math|Conversions|ToTransform(Vector) (Transformation|GetWorldLocation (Variables|Default|GetSpawnLocation)))))