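; A purchasable health station that players buy with points, first advertised as doubling health and afterwards as replenishing it.
; Overlap shows or clears a cost prompt on actors implementing BPI_Score, and CanBuy checks points against Cost.
; Buy sends MaxHealth and the point deduction to the player and plays a sound; the first purchase also switches prompt and price.
; Skull-based life purchases are always refused.
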(event EventBeginPlay
  (Variables|Default|SetDisplay%20String "Hold F To Double Health"))

(event EventTick
  (params (DeltaSeconds :type Float%20%28single-precision%29)))

(event Collision|EventActorEndOverlap
  (params (OtherActor :type Actor%20Object%20Reference))
  (if (Utilities|DoesObjectImplementInterface OtherActor "/Game/Blueprints/Interfaces/BPI_Score.BPI_Score_C")
    (Class|BPIScore|DisplayPrompt(Message) OtherActor)))

(event Collision|EventActorBeginOverlap
  (params (OtherActor :type Actor%20Object%20Reference))
  (if (Utilities|DoesObjectImplementInterface OtherActor "/Game/Blueprints/Interfaces/BPI_Score.BPI_Score_C")
    (Class|BPIScore|DisplayPrompt(Message) OtherActor (Utilities|String|Append (Variables|Default|GetDisplay%20String) " 
Cost [" (Utilities|String|ToString(Integer) (Variables|Default|GetCost)) "]"))))

(event EventBuy
  (params (Player :type Actor%20Object%20Reference))
  (bind _returnvalue (Transformation|GetActorLocation))
  (if (Variables|Default|GetAtMax)
    (Class|BPIScore|SetHealth(Message) Player (Variables|Default|GetMaxHealth))
    (Class|BPIScore|TakePoints(Message) Player (Variables|Default|GetCost))
    (Audio|PlaySoundatLocation "/Game/Free_Sounds_Pack/cue/Magical_Interface_5-1_Cue.Magical_Interface_5-1_Cue" _returnvalue "0, 0, 0" 1.0 1.0 0.0 0 0 0 0)
    (else
      (Class|BPIScore|SetHealth(Message) Player (Variables|Default|GetMaxHealth))
      (Class|BPIScore|TakePoints(Message) Player (Variables|Default|GetCost))
      (Variables|Default|SetAtMax true)
      (Variables|Default|SetDisplay%20String "Hold F To Replenish Health")
      (Variables|Default|SetCost 300)
      (Class|BPIScore|DisplayPrompt(Message) Player (Utilities|String|Append (Variables|Default|GetDisplay%20String) " 
Cost [" (Utilities|String|ToString(Integer) (Variables|Default|GetCost)) "]"))
      (Audio|PlaySoundatLocation "/Game/Free_Sounds_Pack/cue/Magical_Interface_5-1_Cue.Magical_Interface_5-1_Cue" _returnvalue "0, 0, 0" 1.0 1.0 0.0 0 0 0 0))))

(fn ConstructionScript)

(fn CanBuy?
  (params (CurrentPoints :type Integer))
  (return (>= CurrentPoints (Variables|Default|GetCost))))

(fn CanBuyLife?
  (params (Skulls :type Integer))
  (return false))