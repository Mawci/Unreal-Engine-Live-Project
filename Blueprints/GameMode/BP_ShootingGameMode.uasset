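; Game mode for a wave-based shooter that runs enemy waves, wave text and audio cues.
; Each wave randomly picks more Spawn0-tagged spawners, up to a cap, and lights them with staggered explosions.
; A delayed loop spawns BP_Enemy with hand-tuned early-wave difficulty, then scaling health and count, while limiting living enemies to MaxHoard.
; EnemyKilled refills the horde and, when none remain, resets spawners and advances the wave.
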(event Custom|StartGame
  (Utilities|FlowControl|Delay 5.0)
  (Widget|SetVisibility (Variables|Default|GetWave%20Text) "Hidden")
  (CallFunction|SpawnNewWave))

(event Custom|SpawnNewWave
  (bind _current_wave (Variables|Default|GetCurrent%20Wave))
  (CallFunction|SetActiveWaveSpawns)
  (Utilities|FlowControl|Delay (* (Math|Integer|Clamp(Integer) (Variables|Default|GetCurrent%20Wave) 1 (Variables|Default|GetMaxTotalActiveSpawners)) 1.9))
  (switch int _current_wave
    (:Default
      ;[1 1 1] First 6 Rounds Difficulty fixed
      (Variables|Default|SetEnemyHealth (+ (Variables|Default|GetEnemyHealth) 5e+01))
      (Variables|Default|SetEnemySpeed 3e+02)
      (Variables|Default|SetSpawnDelayMin 0.3)
      (Variables|Default|SetSpawnDelayMax 1.5)
      (bind _output_get (Variables|Default|SetTotal%20Enemies (* _current_wave 9))))
    (:1
      (Variables|Default|SetEnemySpeed 85.0)
      (Variables|Default|SetEnemyHealth 5e+01)
      (Variables|Default|SetTotal%20Enemies 6))
    (:2
      (Variables|Default|SetEnemySpeed 9e+01)
      (Variables|Default|SetEnemyHealth 1e+02)
      (Variables|Default|SetTotal%20Enemies 12))
    (:3
      (Variables|Default|SetEnemySpeed 1.5e+02)
      (Variables|Default|SetEnemyHealth 1.5e+02)
      (Variables|Default|SetTotal%20Enemies 20))
    (:4
      (Variables|Default|SetEnemySpeed 175.0)
      (Variables|Default|SetEnemyHealth 2e+02)
      (Variables|Default|SetTotal%20Enemies 30)
      (Variables|Default|SetSpawnDelayMin 0.5)
      (Variables|Default|SetSpawnDelayMax 4.0))
    (:5
      (Variables|Default|SetEnemySpeed 2e+02)
      (Variables|Default|SetEnemyHealth 2.5e+02)
      (Variables|Default|SetTotal%20Enemies 42)
      (Variables|Default|SetSpawnDelayMin 0.4)
      (Variables|Default|SetSpawnDelayMax 3.0))
    (:6
      (Variables|Default|SetEnemySpeed 2.5e+02)
      (Variables|Default|SetEnemyHealth 3e+02)
      (Variables|Default|SetTotal%20Enemies 56)
      (Variables|Default|SetSpawnDelayMin 0.3)
      (Variables|Default|SetSpawnDelayMax 2.0))
    (:7
      (Variables|Default|SetEnemySpeed 3e+02)
      (Variables|Default|SetEnemyHealth 325.0)
      (Variables|Default|SetTotal%20Enemies 60)))
  (Variables|Default|SetRemaining%20Enemies _output_get)
  ;[1 1 1] Add Spawn Enemies Function here and delete this comment
  (Variables|Default|SetCurrentHoard 0)
  (CallFunction|SpawnEnemies))

(event Custom|Enemy%20Killed
  (Math|Integer|DecrementInt (Variables|Default|GetCurrentHoard)
    (:%20%20
      (if (and (Variables|Default|GetisSpawning) (not (!= (Variables|Default|GetTotal%20Enemies) 0)))
        _
        (else
          (CallFunction|SpawnEnemies)))
      (bind _result (Math|Integer|DecrementInt (Variables|Default|GetRemaining%20Enemies))
        (:%20%20
          (if (== _result 0)
            (CallFunction|WaveIncrement)))))))

(event Custom|Wave%20Increment
  (bind _wavecomplete (Variables|Default|GetWaveComplete))
  (Utilities|FlowControl|Delay 2.0)
  (CallFunction|ResetSpawns)
  (Class|AudioComponent|SetPaused _wavecomplete false)
  (Audio|Components|Audio|FadeIn _wavecomplete 0.0 1.0 0.0 "Linear" :!class /Script/Engine.AudioComponent)
  (Audio|Components|Audio|SetVolumeMultiplier _wavecomplete 0.25 :!class /Script/Engine.AudioComponent)
  (Utilities|FlowControl|Delay 4.0)
  (Audio|Components|Audio|FadeOut _wavecomplete 5.0 0.0 "Linear" :!class /Script/Engine.AudioComponent)
  (Math|Integer|IncrementInt (Variables|Default|GetCurrent%20Wave)
    (:%20%20
      (Widget|SetVisibility (Variables|Default|GetWave%20Text) "Visible")
      (Utilities|FlowControl|Delay 5.0)
      (Widget|SetVisibility (Variables|Default|GetWave%20Text) "Hidden")
      (Utilities|FlowControl|Delay 1.0)
      (CallFunction|SpawnNewWave))))

(event Custom|SetActiveWaveSpawns
  (bind _activespawns (Variables|Default|GetActiveSpawns))
  (bind _output_get (Variables|Default|SetTotalActiveSpawners (Math|Integer|Clamp(Integer) (Variables|Default|GetCurrent%20Wave) 1 (Variables|Default|GetMaxTotalActiveSpawners))))
  (bind _output_get_2 (Variables|Default|SetIndex _output_get))
  (Development|PrintString (Utilities|String|Append (Utilities|String|ToString(Integer) _output_get_2) " Spawns to light up"))
  (Utilities|Array|Clear (Variables|Default|GetActiveSpawns))
  (if (> (Variables|Default|GetTotalActiveSpawners) 0) :!label _label
    (bind _output_get_3 (Variables|Default|SettempSpawner (.OutItem (Utilities|Array|Random (Variables|Default|GetAll%20Spawns)))))
    (Utilities|Array|AddUnique (Variables|Default|GetActiveSpawns) _output_get_3)
    (Utilities|Array|RemoveItem (Variables|Default|GetAll%20Spawns) _output_get_3)
    (Math|Integer|DecrementInt (Variables|Default|GetTotalActiveSpawners)
      (:%20%20
        (goto _label)))
    (else
      (if (> (Variables|Default|GetIndex) -1) :!label _label_2
        (Class|BPISpawner|SetActive(Message) (Utilities|Array|Get(acopy) _activespawns (- (Variables|Default|GetIndex) 1)))
        (Development|PrintString (Utilities|String|Append "Size of array " (Utilities|String|ToString(Integer) (Utilities|Array|Length _activespawns))))
        (bind _spawnlocation (Class|BPISpawner|GetLocation(Message) (Utilities|Array|Get(acopy) _activespawns (- (Variables|Default|GetIndex) 1))))
        (Effects|SpawnEmitteratLocation "/Game/StarterContent/Particles/P_Explosion.P_Explosion" (.location _spawnlocation) "0, 0, 0" "5.000000,5.000000,5.000000")
        (bind _result (Math|Integer|DecrementInt (Variables|Default|GetIndex))
          (:%20%20
            (Utilities|FlowControl|Delay 1.8)
            (Development|PrintString (Utilities|String|ToString(Integer) _result))
            (goto _label_2)))))))

(event Custom|ResetSpawns
  (Utilities|Array|Clear (Variables|Default|GetAll%20Spawns))
  (bind _outactors (Actor|GetAllActorswithTag "Spawn0"))
  (bind _output_get (Variables|Default|SetAll%20Spawns _outactors))
  (for _array_element _output_get
    (Class|BPISpawner|SetInactive(Message) _array_element)))

(event Custom|ActivateSpawns)

(event Custom|SpawnEnemies
  ;[1 1 1] Spawning Logic with a max amount of enemies allowed on the map at one time
  (if (not (Variables|Default|GetisSpawning))
    (if (and (!= (Variables|Default|GetTotal%20Enemies) 0) (!= (Variables|Default|GetCurrentHoard) (Variables|Default|GetMaxHoard))) :!label _label
      (Variables|Default|SetisSpawning true)
      (Math|Integer|DecrementInt (Variables|Default|GetTotal%20Enemies)
        (:%20%20
          (Math|Integer|IncrementInt (Variables|Default|GetCurrentHoard)
            (:%20%20
              (bind _spawnlocation (Class|BPISpawner|GetLocation(Message) (.OutItem (Utilities|Array|Random (Variables|Default|GetActiveSpawns)))))
              (bind _returnvalue (Game|SpawnActorfromClass "/Game/Enemy/BP_Enemy.BP_Enemy_C" _spawnlocation "AdjustIfPossibleButAlwaysSpawn" "MultiplyWithRoot" 0 0))
              (Class|BPIDamagable|SetHealth(Message) _returnvalue (Variables|Default|GetEnemyHealth))
              (Class|BPIDamagable|SetSpeed(Message) _returnvalue (Variables|Default|GetEnemySpeed))
              (Utilities|FlowControl|Delay (Math|Random|RandomFloatinRange (Variables|Default|GetSpawnDelayMin) (Variables|Default|GetSpawnDelayMax)))
              (goto _label)))))
      (else
        (Variables|Default|SetisSpawning false)))))

(event EventBeginPlay
  (bind _gamebegin (Variables|Default|GetGameBegin))
  (Class|AudioComponent|SetPaused (Variables|Default|GetWaveComplete) true)
  (bind _returnvalue (UserInterface|CreateWidget "/Game/Blueprints/HUD/UI_WaveText.UI_WaveText_C"))
  (bind _output_get (Variables|Default|SetWave%20Text _returnvalue))
  (UserInterface|Viewport|AddtoViewport _output_get 0)
  (Widget|SetVisibility _output_get "Hidden")
  (Audio|PlaySound2D "/Game/Soundfx/gameAmbience.gameAmbience" 1.0 1.0 0.0 0 0)
  (Audio|Components|Audio|SetVolumeMultiplier _gamebegin 0.05 :!class /Script/Engine.AudioComponent)
  (Audio|Components|Audio|FadeIn _gamebegin 1.0 1.0 0.0 "Linear" :!class /Script/Engine.AudioComponent)
  (Utilities|FlowControl|Delay 5.0)
  (Audio|Components|Audio|FadeOut _gamebegin 5.0 0.0 "Linear" :!class /Script/Engine.AudioComponent)
  (bind _outactors (Actor|GetAllActorswithTag "Spawn0"))
  (Variables|Default|SetAll%20Spawns _outactors)
  (Widget|SetVisibility (Variables|Default|GetWave%20Text) "Visible")
  (CallFunction|StartGame))

(fn ConstructionScript)