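; Weapon upgrade station that sells three escalating tiers of damage multiplier and camo for points.
; Overlap shows or clears the player's prompt, and CanBuy? checks points against Cost and blocks purchases at max level.
; Buy switches on Level, sending player messages to apply a camo taken from that tier's display weapon material, deduct points and refill ammo.
; The first two tiers then raise Cost and update the prompt; CanBuyLife? always returns false.
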(event EventBeginPlay
  (Variables|Default|SetDisplay%20String "Hold  F  To Upgrade Weapon (Doubles Damage)"))

(event EventTick
  (params (DeltaSeconds :type Float%20%28single-precision%29)))

(event Collision|EventActorEndOverlap
  (params (OtherActor :type Actor%20Object%20Reference))
  (if (Utilities|DoesObjectImplementInterface OtherActor "/Game/Blueprints/Interfaces/BPI_Score.BPI_Score_C")
    (Class|BPIScore|DisplayPrompt(Message) OtherActor)))

(event Collision|EventActorBeginOverlap
  (params (OtherActor :type Actor%20Object%20Reference))
  (if (!= (Variables|Default|GetLevel) 3)
    (Class|BPIScore|DisplayPrompt(Message) OtherActor (Utilities|String|Append (Variables|Default|GetDisplay%20String) " 
Cost  [" (Utilities|String|ToString(Integer) (Variables|Default|GetCost)) "]"))
    (else
      (Class|BPIScore|DisplayPrompt(Message) OtherActor "You have the most powerful weapon"))))

(event EventBuy
  (params (Player :type Actor%20Object%20Reference))
  (Audio|PlaySoundatLocation "/Game/Free_Sounds_Pack/cue/Bag_Handle_1-5_Cue.Bag_Handle_1-5_Cue" (Transformation|GetActorLocation) "0, 0, 0" 1.0 1.0 0.0 0 0 0 0)
  (switch int (Variables|Default|GetLevel)
    (:0
      (Class|BPIScore|UpgradeWeapon(Message) Player (Rendering|Material|GetMaterial (Variables|Default|GetWeapon1) 1) 2.0)
      (Class|BPIScore|TakePoints(Message) Player (Variables|Default|GetCost))
      (Class|BPIScore|RefillAmmo(Message) Player)
      (Math|Integer|IncrementInt (Variables|Default|GetLevel)
        (:%20%20
          (Variables|Default|SetDisplay%20String "Hold  F  To Upgrade Weapon (Triples Damage)")
          (Variables|Default|SetCost 4500)
          (Class|BPIScore|DisplayPrompt(Message) Player (Utilities|String|Append (Variables|Default|GetDisplay%20String) " 
Cost  [" (Utilities|String|ToString(Integer) (Variables|Default|GetCost)) "]")))))
    (:1
      (Class|BPIScore|UpgradeWeapon(Message) Player (Rendering|Material|GetMaterial (Variables|Default|GetWeapon2) 1) 3.0)
      (Class|BPIScore|TakePoints(Message) Player (Variables|Default|GetCost))
      (Class|BPIScore|RefillAmmo(Message) Player)
      (Math|Integer|IncrementInt (Variables|Default|GetLevel)
        (:%20%20
          (Variables|Default|SetDisplay%20String "Hold  F  To Upgrade Weapon (Quadruples Damage)")
          (Variables|Default|SetCost 10000)
          (Class|BPIScore|DisplayPrompt(Message) Player (Utilities|String|Append (Variables|Default|GetDisplay%20String) " 
Cost  [" (Utilities|String|ToString(Integer) (Variables|Default|GetCost)) "]")))))
    (:2
      (Class|BPIScore|UpgradeWeapon(Message) Player (Rendering|Material|GetMaterial (Variables|Default|GetWeapon3) 1) 4.0)
      (Class|BPIScore|TakePoints(Message) Player (Variables|Default|GetCost))
      (Class|BPIScore|RefillAmmo(Message) Player)
      (Math|Integer|IncrementInt (Variables|Default|GetLevel)
        (:%20%20
          (bind _output_get (Variables|Default|SetDisplay%20String "You have the most powerful weapon"))
          (Class|BPIScore|DisplayPrompt(Message) Player _output_get))))))

(fn ConstructionScript)

(fn CanBuy?
  (params (CurrentPoints :type Integer))
  (return (and (>= CurrentPoints (Variables|Default|GetCost)) (!= (Variables|Default|GetLevel) 3))))

(fn CanBuyLife?
  (params (Skulls :type Integer))
  (return false))