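; Buyable ammo station that players purchase with points, prompting "Hold F To Buy Ammo" with its cost.
; Overlap begin and end show and clear that prompt on actors implementing BPI_Score.
; CanBuy? compares the player's points to Cost, while CanBuyLife? always refuses skull purchases.
; Buy sends refill-ammo and take-points messages to the player and plays a sound at the station.
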(event EventBeginPlay
  (Variables|Default|SetDisplay%20String "Hold  F  To Buy Ammo"))

(event EventTick
  (params (DeltaSeconds :type Float%20%28single-precision%29)))

(event Collision|EventActorEndOverlap
  (params (OtherActor :type Actor%20Object%20Reference))
  (if (Utilities|DoesObjectImplementInterface OtherActor "/Game/Blueprints/Interfaces/BPI_Score.BPI_Score_C")
    (Class|BPIScore|DisplayPrompt(Message) OtherActor)))

(event Collision|EventActorBeginOverlap
  (params (OtherActor :type Actor%20Object%20Reference))
  (if (Utilities|DoesObjectImplementInterface OtherActor "/Game/Blueprints/Interfaces/BPI_Score.BPI_Score_C")
    (Class|BPIScore|DisplayPrompt(Message) OtherActor (Utilities|String|Append (Variables|Default|GetDisplay%20String) " 
Cost  [" (Utilities|String|ToString(Integer) (Variables|Default|GetCost)) "]"))))

(event EventBuy
  (params (Player :type Actor%20Object%20Reference))
  (Class|BPIScore|RefillAmmo(Message) Player)
  (Class|BPIScore|TakePoints(Message) Player (Variables|Default|GetCost))
  (Audio|PlaySoundatLocation "/Game/Free_Sounds_Pack/cue/Book_Handle_1-5_Cue.Book_Handle_1-5_Cue" (Transformation|GetActorLocation) "0, 0, 0" 1.0 1.0 0.0 0 0 0 0))

(fn ConstructionScript)

(fn CanBuy?
  (params (CurrentPoints :type Integer))
  (return (>= CurrentPoints (Variables|Default|GetCost))))

(fn CanBuyLife?
  (params (Skulls :type Integer))
  (return false))